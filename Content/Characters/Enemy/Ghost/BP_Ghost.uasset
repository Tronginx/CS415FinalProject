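; Ghost enemy that roams around its spawn point, chases the player and deals contact damage on a cooldown.
; An AIState enum drives AI MoveTo events: pawn sensing triggers Chase, and a retriggerable delay issues a return to spawn, then immediately resumes Roam.
; Tick polls the player's Alarm flag, sending the ghost toward the player when within range.
; Incoming damage reduces health and destroys the ghost at zero.
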(event `self.PawnSensing.OnSeePawn`
  (params (Pawn :type "Pawn Object Reference"))
  (cast `/Game/ThirdPerson/Blueprints/BP_ThirdPersonCharacter` Pawn)
  (`|ExecutionSequence`
    (:`then_0`
      (set `self.AIState` "NewEnumerator2")
      (`self.TriggerState`))
    (:`then_1`
      (`KismetSystemLibrary.RetriggerableDelay` 2.0)
      (`self.Return`)
      (set `self.AIState` "NewEnumerator1")
      (`self.TriggerState`))))

(event `self.ReceiveBeginPlay`
  (set `self.SpawnPoint` (`self.K2_GetActorLocation`))
  (`self.TriggerState`))

(event `Roam`
  (`|AIMoveTo` self (`NavigationSystemV1.K2_GetRandomReachablePointInRadius` (`self.SpawnPoint`) 1000.0 null null) null
    (:`OnSuccess`
      _)
    (:`OnFail`
      _))
  (`KismetSystemLibrary.Delay` 1.0)
  (`self.TriggerState`))

(event `Chase Player`
  (`|AIMoveTo` self (0.0 0.0 0.0) (`GameplayStatics.GetPlayerCharacter` 0)))

(event `TriggerState`
  (switch `/Game/Characters/Enemy/Ghost/EAIState` (`self.AIState`)
    (:`NewEnumerator1`
      (`self.Roam`))
    (:`NewEnumerator2`
      (`self.Chase Player`))))

(event `Return`
  (`|AIMoveTo` self (`self.SpawnPoint`) null))

(event `self.ReceiveHit`
  (params (MyComp :type "PrimitiveComponent Object Reference") (Other :type "Actor Object Reference") (OtherComp :type "PrimitiveComponent Object Reference") (bSelfMoved :type Boolean) (HitLocation :type "Vector Structure") (HitNormal :type "Vector Structure") (NormalImpulse :type "Vector Structure") (Hit :type "HitResult Structure (by ref)"))
  (bind _asbp_third_person_character (cast `/Game/ThirdPerson/Blueprints/BP_ThirdPersonCharacter` Other))
  (if (`self.CanDamage`)
    (set `self.CanDamage` false)
    (`GameplayStatics.ApplyDamage` _asbp_third_person_character 10.0)
    (`KismetSystemLibrary.Delay` 1.0)
    (set `self.CanDamage` true)))

(event `self.ReceiveAnyDamage`
  (params (Damage :type "Float (single-precision)") (DamageType :type "DamageType Object Reference") (InstigatedBy :type "Controller Object Reference") (DamageCauser :type "Actor Object Reference"))
  (set `self.CurrentHealth` (- (`self.CurrentHealth`) Damage))
  (if (<= (`self.CurrentHealth`) 0.0)
    (`self.K2_DestroyActor`)))

(event `self.ReceiveTick`
  (params (DeltaSeconds :type "Float (single-precision)"))
  (bind _asbp_third_person_character (cast `/Game/ThirdPerson/Blueprints/BP_ThirdPersonCharacter` (`GameplayStatics.GetPlayerPawn` 0)))
  (if (`/Game/ThirdPerson/Blueprints/BP_ThirdPersonCharacter.Alarm` _asbp_third_person_character)
    (`self.Alarmed`)))

(event `Alarmed`
  (bind _asbp_third_person_character (cast `/Game/ThirdPerson/Blueprints/BP_ThirdPersonCharacter` (`GameplayStatics.GetPlayerPawn` 0)))
  (if (<= (`KismetMathLibrary.Vector_Distance` (`self.K2_GetActorLocation` _asbp_third_person_character) (`self.K2_GetActorLocation`)) 3000.0)
    (`|AIMoveTo` self (0.0 0.0 0.0) _asbp_third_person_character)))

(fn `UserConstructionScript`)