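; BP_Exploder is an enemy that roams around its spawn point and chases the player on sight, exploding on contact or death.
; An AIState switch drives AIMoveTo for roaming or chasing, with pawn sensing triggering chase.
; A retriggerable delay after the last sighting calls Return to spawn, then immediately resumes roaming.
; Explode damages the player if within range, plays sound and particle effects, then destroys the actor.
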(event `self.PawnSensing.OnSeePawn`
  (params (Pawn :type "Pawn Object Reference"))
  (cast `/Game/ThirdPerson/Blueprints/BP_ThirdPersonCharacter` Pawn)
  (`|ExecutionSequence`
    (:`then_0`
      (set `self.AIState` "NewEnumerator2")
      (`self.TriggerState`))
    (:`then_1`
      (`KismetSystemLibrary.RetriggerableDelay` 2.0)
      (`self.Return`)
      (set `self.AIState` "NewEnumerator1")
      (`self.TriggerState`))))

(event `self.ReceiveBeginPlay`
  (set `self.SpawnPoint` (`self.K2_GetActorLocation`))
  (`self.TriggerState`))

(event `Roam`
  (`|AIMoveTo` self (`NavigationSystemV1.K2_GetRandomReachablePointInRadius` (`self.SpawnPoint`) 1000.0 null null) null
    (:`OnSuccess`
      _)
    (:`OnFail`
      _))
  (`KismetSystemLibrary.Delay` 1.0)
  (`self.TriggerState`))

(event `Chase Player`
  (`|AIMoveTo` self (0.0 0.0 0.0) (`GameplayStatics.GetPlayerCharacter` 0)))

(event `TriggerState`
  (switch `/Game/Characters/Enemy/Exploder/EAIState_Exploder` (`self.AIState`)
    (:`NewEnumerator1`
      (`self.Roam`))
    (:`NewEnumerator2`
      (`self.Chase Player`))))

(event `Return`
  (`|AIMoveTo` self (`self.SpawnPoint`) null))

(event `self.ReceiveHit`
  (params (MyComp :type "PrimitiveComponent Object Reference") (Other :type "Actor Object Reference") (OtherComp :type "PrimitiveComponent Object Reference") (bSelfMoved :type Boolean) (HitLocation :type "Vector Structure") (HitNormal :type "Vector Structure") (NormalImpulse :type "Vector Structure") (Hit :type "HitResult Structure (by ref)"))
  (cast `/Game/ThirdPerson/Blueprints/BP_ThirdPersonCharacter` Other)
  (`self.Explode`))

(event `self.ReceiveAnyDamage`
  (params (Damage :type "Float (single-precision)") (DamageType :type "DamageType Object Reference") (InstigatedBy :type "Controller Object Reference") (DamageCauser :type "Actor Object Reference"))
  (set `self.CurrentHealth` (- (`self.CurrentHealth`) Damage))
  (if (<= (`self.CurrentHealth`) 0.0)
    (`self.Explode`)))

(fn `Explode`
  (bind _returnvalue (`self.K2_GetActorLocation`))
  (if (not (> (`KismetMathLibrary.VSize` (- (`self.K2_GetActorLocation` (`GameplayStatics.GetPlayerPawn` 0)) (`self.K2_GetActorLocation`))) 300.0))
    (`GameplayStatics.ApplyDamage` (`GameplayStatics.GetPlayerPawn` 0) 50.0))
  (`GameplayStatics.PlaySoundAtLocation` "/Game/StarterContent/Audio/Explosion01.Explosion01" _returnvalue (struct) 1.0 1.0 0.0 null null null null)
  (`GameplayStatics.SpawnEmitterAtLocation` "/Game/StarterContent/Particles/P_Explosion.P_Explosion" _returnvalue)
  (`self.K2_DestroyActor`))

(fn `UserConstructionScript`)