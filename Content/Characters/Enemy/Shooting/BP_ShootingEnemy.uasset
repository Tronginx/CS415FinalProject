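; Shooting enemy that roams around its spawn point, fires bullets at a seen player and deals damage on hit.
; PawnSensing switches an AIState-driven loop to shooting, and a retriggerable delay sends it back to roaming after sight lapses.
; Tick either halts and faces the player while staring or pursues a nearby player whose Alarm is set.
; Damage updates a widget health bar, and death triggers an explosion.
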(event `self.PawnSensing.OnSeePawn`
  (params (Pawn :type "Pawn Object Reference"))
  (cast `/Game/ThirdPerson/Blueprints/BP_ThirdPersonCharacter` Pawn)
  (`|ExecutionSequence`
    (:`then_0`
      (set `self.AIState` "NewEnumerator2")
      (`KismetSystemLibrary.Delay` 0.5)
      (`self.TriggerState`))
    (:`then_1`
      (`KismetSystemLibrary.RetriggerableDelay` 2.0)
      (`self.Return`)
      (set `self.AIState` "NewEnumerator1")
      (`self.TriggerState`))))

(event `self.ReceiveBeginPlay`
  (set `self.SpawnPoint` (`self.K2_GetActorLocation`))
  (`self.TriggerState`)
  (`self.UpdateHealthUI`))

(event `Roam`
  (`|AIMoveTo` self (`NavigationSystemV1.K2_GetRandomReachablePointInRadius` (`self.SpawnPoint`) 1000.0 null null) null
    (:`OnSuccess`
      _)
    (:`OnFail`
      _))
  (`KismetSystemLibrary.Delay` 1.0)
  (`self.TriggerState`))

(event `ShootPlayer`
  (`GameplayStatics.PlaySoundAtLocation` "/Game/ThirdPerson/Assets/gunshot2.gunshot2" (`SceneComponent.K2_GetComponentLocation` (`self.BulletSpawn`)) (struct) 1.0 1.0 0.0 null null null null)
  (`|SpawnActorFromClass` "/Game/Characters/Enemy/Shooting/BP_Bullet.BP_Bullet_C" (`SceneComponent.K2_GetComponentToWorld` (`self.BulletSpawn`)) "AlwaysSpawn" "MultiplyWithRoot" null null))

(event `TriggerState`
  (switch `/Game/Characters/Enemy/Shooting/EAIState_Shooting` (`self.AIState`)
    (:`NewEnumerator1`
      (`self.Roam`)
      (set `self.Staring` false))
    (:`NewEnumerator2`
      (`self.ShootPlayer`)
      (set `self.Staring` true))))

(event `Return`
  (`|AIMoveTo` self (`self.SpawnPoint`) null))

(event `self.ReceiveHit`
  (params (MyComp :type "PrimitiveComponent Object Reference") (Other :type "Actor Object Reference") (OtherComp :type "PrimitiveComponent Object Reference") (bSelfMoved :type Boolean) (HitLocation :type "Vector Structure") (HitNormal :type "Vector Structure") (NormalImpulse :type "Vector Structure") (Hit :type "HitResult Structure (by ref)"))
  (bind _asbp_third_person_character (cast `/Game/ThirdPerson/Blueprints/BP_ThirdPersonCharacter` Other))
  (`GameplayStatics.ApplyDamage` _asbp_third_person_character 10.0))

(event `self.ReceiveAnyDamage`
  (params (Damage :type "Float (single-precision)") (DamageType :type "DamageType Object Reference") (InstigatedBy :type "Controller Object Reference") (DamageCauser :type "Actor Object Reference"))
  (bind _returnvalue (`self.K2_GetActorLocation`))
  (set `self.CurrentHealth` (- (`self.CurrentHealth`) Damage))
  (`self.UpdateHealthUI`)
  (if (<= (`self.CurrentHealth`) 0.0)
    (`self.K2_DestroyActor`)
    (`GameplayStatics.SpawnEmitterAtLocation` "/Game/Realistic_Starter_VFX_Pack_Vol2/Particles/Explosion/P_Explosion_Big_A.P_Explosion_Big_A" _returnvalue)
    (`GameplayStatics.PlaySoundAtLocation` "/Game/Free_Sounds_Pack/wav/Explosion_Large_1-1.Explosion_Large_1-1" _returnvalue (struct) 1.0 1.0 0.0 null null null null)))

(event `Stare`
  (`MovementComponent.StopMovementImmediately` (`self.CharacterMovement`))
  (`self.K2_SetActorRotation` (`KismetMathLibrary.MakeRotFromX` (`KismetMathLibrary.Normal` (`KismetMathLibrary.MakeVector` (.x (- (`self.K2_GetActorLocation` (`GameplayStatics.GetPlayerPawn` 0)) (`self.K2_GetActorLocation`))) (.y (- (`self.K2_GetActorLocation` (`GameplayStatics.GetPlayerPawn` 0)) (`self.K2_GetActorLocation`))))))))

(event `self.ReceiveTick`
  (params (DeltaSeconds :type "Float (single-precision)"))
  (if (`self.Staring`)
    (`self.Stare`)
    (else
      (bind _asbp_third_person_character (cast `/Game/ThirdPerson/Blueprints/BP_ThirdPersonCharacter` (`GameplayStatics.GetPlayerPawn` 0)))
      (if (`/Game/ThirdPerson/Blueprints/BP_ThirdPersonCharacter.Alarm` _asbp_third_person_character)
        (`self.Alarmed`)))))

(event `Alarmed`
  (bind _asbp_third_person_character (cast `/Game/ThirdPerson/Blueprints/BP_ThirdPersonCharacter` (`GameplayStatics.GetPlayerPawn` 0)))
  (if (<= (`KismetMathLibrary.Vector_Distance` (`self.K2_GetActorLocation` _asbp_third_person_character) (`self.K2_GetActorLocation`)) 3000.0)
    (`|AIMoveTo` self (0.0 0.0 0.0) _asbp_third_person_character)))

(fn `UpdateHealthUI`
  (bind _health_bar (`self.Health Bar`))
  (bind _aswb_enemy_health_bar (cast `/Game/Characters/Enemy/WB_EnemyHealthBar` (`WidgetComponent.GetWidget` (`self.Health Bar`))))
  (`ProgressBar.SetPercent` (`/Game/Characters/Enemy/WB_EnemyHealthBar.HealthBar` _aswb_enemy_health_bar) (/ (`self.CurrentHealth`) (`self.MaxHealth`)))
  (`SceneComponent.K2_SetWorldRotation` _health_bar (`KismetMathLibrary.FindLookAtRotation` (`SceneComponent.K2_GetComponentLocation` _health_bar) (`SceneComponent.K2_GetComponentLocation` (`PlayerCameraManager.TransformComponent` (`GameplayStatics.GetPlayerCameraManager` 0)))) false false))

(fn `UserConstructionScript`)