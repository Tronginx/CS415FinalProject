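; BP_Follower is a companion pawn that wanders around the player and closes in when left behind.
; A two-state loop (Roam, Follow) dispatched by TriggerState issues AIMoveTo calls to random reachable points around the player, wide for Roam and tight for Follow.
; Tick updates the player distance, which Roam checks after a short delay to switch to Follow.
; Follow switches back to Roam from its move's Then output, with no delay.
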(event `TriggerState`
  (switch `/Game/Characters/Follower/EAIState_Follower` (`self.AIState`)
    (:`NewEnumerator0`
      (`self.Roam`))
    (:`NewEnumerator1`
      (`self.Follow`))))

(event `self.ReceiveBeginPlay`
  (`self.TriggerState`))

(event `Roam`
  (bind _asbp_third_person_character (cast `/Game/ThirdPerson/Blueprints/BP_ThirdPersonCharacter` (`GameplayStatics.GetPlayerPawn` 0)))
  (`|AIMoveTo` self (`NavigationSystemV1.K2_GetRandomReachablePointInRadius` (`self.K2_GetActorLocation` _asbp_third_person_character) 300.0 null null) null
    (:`then`
      (`KismetSystemLibrary.Delay` 1.0)
      (if (> (`self.PlayerDistance`) 500.0)
        (set `self.AIState` "NewEnumerator1"))
      (`self.TriggerState`))))

(event `Follow`
  (bind _asbp_third_person_character (cast `/Game/ThirdPerson/Blueprints/BP_ThirdPersonCharacter` (`GameplayStatics.GetPlayerPawn` 0)))
  (`|AIMoveTo` self (`NavigationSystemV1.K2_GetRandomReachablePointInRadius` (`self.K2_GetActorLocation` _asbp_third_person_character) 50.0 null null) null
    (:`then`
      (set `self.AIState` "NewEnumerator0")
      (`self.TriggerState`))))

(event `self.ReceiveTick`
  (params (DeltaSeconds :type "Float (single-precision)"))
  (bind _asbp_third_person_character (cast `/Game/ThirdPerson/Blueprints/BP_ThirdPersonCharacter` (`GameplayStatics.GetPlayerPawn` 0)))
  (set `self.PlayerDistance` (`KismetMathLibrary.Vector_Distance` (`self.K2_GetActorLocation` _asbp_third_person_character) (`self.K2_GetActorLocation`))))

(fn `UserConstructionScript`)