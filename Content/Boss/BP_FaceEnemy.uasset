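; Boss face enemy that fires a continuous laser from its Cube mesh when ShootLaser is called.
; ShootLaser flashes the cube red through a looping timer and dynamic material as a telegraph, then enables EmitLaser after a delay.
; While enabled, Tick spawns beam and impact particles once via DoOnce, line-traces along the cube's forward vector, and damages BP_ThirdPersonCharacter every frame it is hit.
; StopShoot resets the color and flag, letting Tick clear the effects.
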(event `StopShoot`
  (`self.ChangeColor` (make `Color` 0 0 0 100))
  (set `self.EmitLaser` false))

(event `ShineRed`
  (`KismetSystemLibrary.Delay` 0.5)
  (`self.ChangeColor` (make `Color` 0 0 0 100))
  (`KismetSystemLibrary.Delay` 0.5)
  (`self.ChangeColor` (make `Color` 0 0 255 100)))

(event `ShootLaser`
  (`KismetSystemLibrary.K2_SetTimer` null "ShineRed" 1.0 true false -1.0)
  (`KismetSystemLibrary.Delay` 3.0)
  (`KismetSystemLibrary.K2_PauseTimer` null "ShineRed")
  (set `self.EmitLaser` true))

(event `self.ReceiveBeginPlay`)

(event `self.ReceiveTick`
  (params (DeltaSeconds :type "Float (single-precision)"))
  (bind _cube (`self.Cube`))
  (bind _laserhit (`self.LaserHit`))
  (bind _laserhit_2 (`self.LaserHit`))
  (bind _laserparticle (`self.LaserParticle`))
  (bind _returnvalue (`SceneComponent.K2_GetComponentLocation` _cube))
  (bind _returnvalue_2 (+ _returnvalue (* (`SceneComponent.GetForwardVector` _cube) 10000)))
  (if (`self.EmitLaser`)
    (`|ExecutionSequence`
      (:`then_0`
        (`/Engine/EditorBlueprintResources/StandardMacros.DoOnce` false :!label _label
          (:`Completed`
            (bind _returnvalue_3 (`GameplayStatics.SpawnEmitterAttached` "/Game/Boss/Particles/P_EnemyLaser.P_EnemyLaser" (`self.Cube`) "None" (0.0 0.0 0.0) (struct) (1.5 1.5 1.5)))
            (set `self.LaserParticle` _returnvalue_3)
            (set `self.LaserSpawn` true))))
      (:`then_1`
        (`/Engine/EditorBlueprintResources/StandardMacros.DoOnce` false :!label _label_2
          (:`Completed`
            (bind _returnvalue_4 (`GameplayStatics.SpawnEmitterAtLocation` "/Game/Boss/Particles/P_LaserHit3.P_LaserHit3" (0.0 0.0 0.0) (struct) (1.5 1.5 1.5)))
            (set `self.LaserHit` _returnvalue_4)
            (set `self.LaserHitSpawn` true))))
      (:`then_2`
        (bind (_outhit _returnvalue_5) (`KismetSystemLibrary.LineTraceSingle` _returnvalue _returnvalue_2 "TraceTypeQuery1"))
        (if _returnvalue_5
          (`SceneComponent.SetVisibility` _laserhit_2 true false)
          (bind (_bblockinghit _binitialoverlap _time _distance _location _impactpoint _normal _impactnormal _physmat _hitactor) (`GameplayStatics.BreakHitResult` _outhit))
          (`SceneComponent.K2_SetWorldLocation` _laserhit_2 _location false false)
          (bind _asbp_third_person_character (cast `/Game/ThirdPerson/Blueprints/BP_ThirdPersonCharacter` _hitactor))
          (`GameplayStatics.ApplyDamage` _asbp_third_person_character 2.0)
          (else
            (`SceneComponent.SetVisibility` _laserhit_2 false false))))
      (:`then_3`
        (`ParticleSystemComponent.SetBeamSourcePoint` _laserparticle 0 _returnvalue 0)
        (`ParticleSystemComponent.SetBeamEndPoint` _laserparticle 0 _returnvalue_2)))
    (else
      (`|ExecutionSequence`
        (:`then_0`
          (goto _label :!via `Reset`))
        (:`then_1`
          (goto _label_2 :!via `Reset`))
        (:`then_2`
          (if (`self.LaserSpawn`)
            (set `self.LaserSpawn` false)
            (`ActorComponent.K2_DestroyComponent` (`self.LaserParticle`))))
        (:`then_3`
          (if (`self.LaserHitSpawn`)
            (`/Engine/EditorBlueprintResources/StandardMacros.IsValid` _laserhit
              (:`Is Valid`
                (`ActorComponent.Deactivate` _laserhit)
                (set `self.LaserHitSpawn` false)))))))))

(fn `ChangeColor`
  (params (NewParam :type "Color Structure"))
  (bind _returnvalue (`PrimitiveComponent.CreateDynamicMaterialInstance` (`self.Cube`) 0 "/Game/Boss/Meshes/MI_CubeEnemy.MI_CubeEnemy" "None"))
  (`MaterialInstanceDynamic.SetVectorParameterValue` _returnvalue "Color" (`KismetMathLibrary.Conv_ColorToLinearColor` NewParam)))

(fn `UserConstructionScript`)