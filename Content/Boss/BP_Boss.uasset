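; BP_Boss is a rotating, vertically drifting boss assembled from face, edge and vertex child actors, with a health bar after activation.
; Tick calls Attack, whose Delay paces random picks between laser, bomb, shield and funnel attacks, each relayed to matching child actors with new spin speeds.
; While shielded, hits heal it instead of hurting.
; Depleting its health destroys it and shows the win UI.
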(event `self.ReceiveAnyDamage`
  (params (Damage :type "Float (single-precision)") (DamageType :type "DamageType Object Reference") (InstigatedBy :type "Controller Object Reference") (DamageCauser :type "Actor Object Reference"))
  (bind _status (`self.Status`))
  (if (>= _status 0)
    (if (== _status 3)
      (`GameplayStatics.PlaySoundAtLocation` "/Game/Free_Sounds_Pack/wav/Special_Collectible_26-1.Special_Collectible_26-1" (0.0 0.0 0.0) (struct) 1.0 1.0 0.0 null null null null)
      (set `self.HealthPoint` (`KismetMathLibrary.FClamp` (+ (`self.HealthPoint`) 50.0) 0.0 (`self.MaxHealthPoint`)))
      (else
        (bind _output_get (set `self.HealthPoint` (- (`self.HealthPoint`) Damage)))
        (if (<= _output_get 0.0)
          (`self.K2_DestroyActor`)
          (`Widget.RemoveFromParent` (`self.BossHealthBar`))
          (bind _returnvalue (`|CreateWidget` "/Game/ThirdPerson/UI/GameWinUI.GameWinUI_C"))
          (`UserWidget.AddToViewport` _returnvalue 0))))))

(event `Protect`
  (params (Protecting :type Boolean))
  (bind _shield (`self.Shield`))
  (if Protecting
    (`SceneComponent.K2_SetRelativeTransform` _shield (`KismetMathLibrary.MakeTransform` (0.0 0.0 0.0) (struct) (7.0 7.0 7.0)) false false)
    (`SceneComponent.SetVisibility` _shield true false)
    (else
      (`SceneComponent.K2_SetRelativeTransform` _shield (`KismetMathLibrary.MakeTransform` (0.0 0.0 0.0)) false false)
      (`SceneComponent.SetVisibility` _shield false false))))

(event `self.ReceiveBeginPlay`
  (`SceneComponent.SetVisibility` (`self.Shield`) false false))

(event `self.ReceiveTick`
  (params (DeltaSeconds :type "Float (single-precision)"))
  (if (>= (`self.Status`) 0)
    (`SceneComponent.K2_AddLocalRotation` (`self.DefaultSceneRoot`) (`KismetMathLibrary.MakeRotator` (`self.RotationSpeedX`) (`self.RotationSpeedY`) (`self.RotationSpeedZ`)) false false)
    (`self.K2_AddActorWorldOffset` (`KismetMathLibrary.MakeVector` 0.0 0.0 (`self.MovementSpeedZ`)))
    (`self.Attack`)
    (`KismetSystemLibrary.Delay` 3.0)
    (`self.SetMovementSpeed`)))

(event `Attack`
  (bind _childactors (`self.GetAllChildActors` true))
  (`KismetSystemLibrary.Delay` (`self.DelayTime`))
  (set `self.Status` 0)
  (`self.StopCubeActions`)
  (switch `int` (`KismetMathLibrary.RandomInteger` 4)
    (:`0`
      (for _array_element _childactors
        (bind _asbp_face_enemy (cast `/Game/Boss/BP_FaceEnemy` _array_element))
        (`/Game/Boss/BP_FaceEnemy.ShootLaser` _asbp_face_enemy)
        (set `self.DelayTime` 5.0)
        (`self.SetRandomRotation` 5.0)))
    (:`1`
      (for _array_element_2 _childactors
        (bind _asbp_edge_enemy (cast `/Game/Boss/BP_EdgeEnemy` _array_element_2))
        (`/Game/Boss/BP_EdgeEnemy.ShootBomb` _asbp_edge_enemy)
        (set `self.DelayTime` 5.0)
        (`self.SetRandomRotation` -5.0)))
    (:`2`
      (for _array_element_3 _childactors
        (bind _asbp_vertex_cube (cast `/Game/Boss/BP_VertexCube` _array_element_3))
        (`/Game/Boss/BP_VertexCube.Protect` _asbp_vertex_cube)
        (set `self.DelayTime` 10.0)
        (`self.SetRandomRotation` 2.0)
        (`KismetSystemLibrary.Delay` 3.0)
        (`self.Protect` true)
        (set `self.Status` 3)))
    (:`3`
      (for _array_element_4 _childactors
        (bind _asbp_vertex_cube_2 (cast `/Game/Boss/BP_VertexCube` _array_element_4))
        (`/Game/Boss/BP_VertexCube.Funnel` _asbp_vertex_cube_2)
        (set `self.DelayTime` 7.0)
        (`self.SetRandomRotation` -2.0)))))

(event `SetMovementSpeed`
  (bind (_returnvalue_x _returnvalue_y _returnvalue_z) (`KismetMathLibrary.BreakVector` (`self.K2_GetActorLocation`)))
  (bind _returnvalue (`KismetMathLibrary.RandomFloat`))
  (if (> _returnvalue_z 1200.0)
    (set `self.MovementSpeedZ` (* _returnvalue -10.0) :!label _label)
    (else
      (if (< _returnvalue_z 0.0)
        _
        (elif (`KismetMathLibrary.RandomBool`)
          _
          (else
            (goto _label))))
      (set `self.MovementSpeedZ` (* _returnvalue 10.0)))))

(fn `Activate`
  (set `self.Status` 0)
  (bind _returnvalue (`|CreateWidget` "/Game/ThirdPerson/UI/WB_BossHealthBar.WB_BossHealthBar_C"))
  (bind _output_get (set `self.BossHealthBar` _returnvalue))
  (`UserWidget.AddToViewport` _output_get 0))

(fn `SetRandomRotation`
  (params (NewParam :type "Float (double-precision)"))
  (set `self.RotationSpeedX` (* (`KismetMathLibrary.RandomFloat`) NewParam))
  (set `self.RotationSpeedY` (* (`KismetMathLibrary.RandomFloat`) NewParam))
  (set `self.RotationSpeedZ` (* (`KismetMathLibrary.RandomFloat`) NewParam)))

(fn `StopCubeActions`
  (for _array_element (`self.GetAllChildActors` true)
    (bind _asbp_edge_enemy (cast `/Game/Boss/BP_EdgeEnemy` _array_element)
      (:`then`
        (`/Game/Boss/BP_EdgeEnemy.StopShoot` _asbp_edge_enemy))
      (:`CastFailed`
        (bind _asbp_face_enemy (cast `/Game/Boss/BP_FaceEnemy` _array_element)
          (:`then`
            (`/Game/Boss/BP_FaceEnemy.StopShoot` _asbp_face_enemy))
          (:`CastFailed`
            (bind _asbp_vertex_cube (cast `/Game/Boss/BP_VertexCube` _array_element))
            (`/Game/Boss/BP_VertexCube.StopActions` _asbp_vertex_cube)
            (`self.Protect` false)))))))

(fn `UserConstructionScript`)