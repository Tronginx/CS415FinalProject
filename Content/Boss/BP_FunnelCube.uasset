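; BP_FunnelCube is an enemy cube that roams once near its spawn point, then repeatedly chases the player and fires a laser.
; An AIState switch drives movement; each chase cycle flashes material color, toggles EmitLaser and costs the cube health until destroyed.
; Tick runs the laser, using DoOnce-gated beam and impact particles plus a forward line trace that damages the player every frame it hits.
; Incoming damage can also destroy it.
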(event `self.ReceiveAnyDamage`
  (params (Damage :type "Float (single-precision)") (DamageType :type "DamageType Object Reference") (InstigatedBy :type "Controller Object Reference") (DamageCauser :type "Actor Object Reference"))
  (bind _output_get (set `self.HealthPoint` (- (`self.HealthPoint`) Damage)))
  (if (<= _output_get 0.0)
    (`self.K2_DestroyActor`)))

(event `self.ReceiveBeginPlay`
  (set `self.SpawnPoint` (`self.K2_GetActorLocation`))
  (`self.TriggerState`)
  (`self.ChangeColor` (make `Color` 0 95 255 100)))

(event `self.ReceiveTick`
  (params (DeltaSeconds :type "Float (single-precision)"))
  (`self.Laser` 0.0))

(event `Roam`
  (`|AIMoveTo` self (`NavigationSystemV1.K2_GetRandomReachablePointInRadius` (`self.SpawnPoint`) 400.0 null null) null 50.0
    (:`OnSuccess`
      _)
    (:`OnFail`
      _))
  (`KismetSystemLibrary.Delay` 0.5)
  (set `self.AIState` "NewEnumerator2")
  (`self.TriggerState`))

(event `Chase`
  (bind _returnvalue (`GameplayStatics.GetPlayerCharacter` 0))
  (`|AIMoveTo` self (0.0 0.0 0.0) _returnvalue 200.0
    (:`then`
      (`self.K2_SetActorRotation` (`KismetMathLibrary.FindLookAtRotation` (`self.K2_GetActorLocation`) (`self.K2_GetActorLocation` _returnvalue))))
    (:`OnSuccess`
      (`KismetSystemLibrary.RetriggerableDelay` 1.0 :!label _label)
      (`self.ShootLaser`)
      (`KismetSystemLibrary.Delay` 3.0)
      (bind _output_get (set `self.HealthPoint` (- (`self.HealthPoint`) 5.0)))
      (if (> _output_get 0.0)
        (`self.TriggerState`)
        (else
          (`self.K2_DestroyActor`))))
    (:`OnFail`
      (goto _label))))

(event `TriggerState`
  (switch `/Game/Characters/Enemy/Ghost/EAIState` (`self.AIState`)
    (:`NewEnumerator1`
      (`self.Roam`))
    (:`NewEnumerator2`
      (`self.Chase`))))

(event `ShootLaser`
  (`self.ChangeColor` (make `Color` 0 0 0 100))
  (`KismetSystemLibrary.Delay` 0.5)
  (`self.ChangeColor` (make `Color` 0 95 255 100))
  (set `self.EmitLaser` true)
  (`KismetSystemLibrary.Delay` 1.0)
  (set `self.EmitLaser` false)
  (`self.ChangeColor` (make `Color` 0 0 0 100)))

(event `Laser`
  (params (DeltaSeconds :type "Float (single-precision)"))
  (bind _laserhit (`self.LaserHit`))
  (bind _laserhit_2 (`self.LaserHit`))
  (bind _laserparticle (`self.LaserParticle`))
  (bind _sphere (`self.Sphere`))
  (bind _returnvalue (`SceneComponent.K2_GetComponentLocation` _sphere))
  (bind _returnvalue_2 (+ _returnvalue (* (`SceneComponent.GetForwardVector` _sphere) 10000)))
  (if (`self.EmitLaser`)
    (`|ExecutionSequence`
      (:`then_0`
        (`/Engine/EditorBlueprintResources/StandardMacros.DoOnce` false :!label _label_2
          (:`Completed`
            (bind _returnvalue_3 (`GameplayStatics.SpawnEmitterAttached` "/Game/Boss/Particles/P_EnemyLaser.P_EnemyLaser" (`self.Sphere`) "None" (0.0 0.0 0.0) (struct) (1.5 1.5 1.5)))
            (set `self.LaserParticle` _returnvalue_3)
            (set `self.LaserSpawn` true))))
      (:`then_1`
        (`/Engine/EditorBlueprintResources/StandardMacros.DoOnce` false :!label _label_3
          (:`Completed`
            (bind _returnvalue_4 (`GameplayStatics.SpawnEmitterAtLocation` "/Game/Boss/Particles/P_LaserHit3.P_LaserHit3" (0.0 0.0 0.0) (struct) (1.5 1.5 1.5)))
            (set `self.LaserHit` _returnvalue_4)
            (set `self.LaserHitSpawn` true))))
      (:`then_2`
        (bind (_outhit _returnvalue_5) (`KismetSystemLibrary.LineTraceSingle` _returnvalue _returnvalue_2 "TraceTypeQuery1"))
        (if _returnvalue_5
          (`SceneComponent.SetVisibility` _laserhit_2 true false)
          (bind (_bblockinghit _binitialoverlap _time _distance _location _impactpoint _normal _impactnormal _physmat _hitactor) (`GameplayStatics.BreakHitResult` _outhit))
          (`SceneComponent.K2_SetWorldLocation` _laserhit_2 _location false false)
          (bind _asbp_third_person_character (cast `/Game/ThirdPerson/Blueprints/BP_ThirdPersonCharacter` _hitactor))
          (`GameplayStatics.ApplyDamage` _asbp_third_person_character 0.5)
          (else
            (`SceneComponent.SetVisibility` _laserhit_2 false false))))
      (:`then_3`
        (`ParticleSystemComponent.SetBeamSourcePoint` _laserparticle 0 _returnvalue 0)
        (`ParticleSystemComponent.SetBeamEndPoint` _laserparticle 0 _returnvalue_2)))
    (else
      (`|ExecutionSequence`
        (:`then_0`
          (goto _label_2 :!via `Reset`))
        (:`then_1`
          (goto _label_3 :!via `Reset`))
        (:`then_2`
          (if (`self.LaserSpawn`)
            (set `self.LaserSpawn` false)
            (`ActorComponent.K2_DestroyComponent` (`self.LaserParticle`))))
        (:`then_3`
          (if (`self.LaserHitSpawn`)
            (`/Engine/EditorBlueprintResources/StandardMacros.IsValid` _laserhit
              (:`Is Valid`
                (`ActorComponent.Deactivate` _laserhit)
                (set `self.LaserHitSpawn` false)))))))))

(fn `ChangeColor`
  (params (NewParam :type "Color Structure"))
  (bind _returnvalue (`PrimitiveComponent.CreateDynamicMaterialInstance` (`self.Mesh`) 0 "/Game/Boss/Meshes/MI_CubeEnemy.MI_CubeEnemy" "None"))
  (`MaterialInstanceDynamic.SetVectorParameterValue` _returnvalue "Color" (`KismetMathLibrary.Conv_ColorToLinearColor` NewParam)))

(fn `UserConstructionScript`)