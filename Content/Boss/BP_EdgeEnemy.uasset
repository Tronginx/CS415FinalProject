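; BP_EdgeEnemy is a cube boss-fight enemy that telegraphs, then repeatedly spawns lightning bombs.
; ShootBomb loops a timer that blinks the cube yellow through a dynamic material's Color parameter, then pauses it and enables emission.
; While emission is on, Tick spawns BP_LightningBomb at two arrow components, using latent Delays to throttle and stagger spawns.
; StopShoot resets the color and clears the emission flag.
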(event `StopShoot`
  (`self.ChangeColor` (make `Color` 0 0 0 100))
  (set `self.EmitBomb` false))

(event `ShineYellow`
  (`KismetSystemLibrary.Delay` 0.5)
  (`self.ChangeColor` (make `Color` 0 0 0 100))
  (`KismetSystemLibrary.Delay` 0.5)
  (`self.ChangeColor` (make `Color` 0 255 255 100)))

(event `ShootBomb`
  (`KismetSystemLibrary.K2_SetTimer` null "ShineYellow" 1.0 true false -1.0)
  (`KismetSystemLibrary.Delay` 3.0)
  (`KismetSystemLibrary.K2_PauseTimer` null "ShineYellow")
  (set `self.EmitBomb` true))

(event `self.ReceiveBeginPlay`)

(event `self.ReceiveTick`
  (params (DeltaSeconds :type "Float (single-precision)"))
  (if (`self.EmitBomb`)
    (`KismetSystemLibrary.Delay` 0.5)
    (`|SpawnActorFromClass` "/Game/Boss/BP_LightningBomb.BP_LightningBomb_C" (`SceneComponent.K2_GetComponentToWorld` (`self.ArrowX`)) "AlwaysSpawn" "MultiplyWithRoot" null null)
    (`KismetSystemLibrary.Delay` 0.5)
    (`|SpawnActorFromClass` "/Game/Boss/BP_LightningBomb.BP_LightningBomb_C" (`SceneComponent.K2_GetComponentToWorld` (`self.ArrowY`)) "AlwaysSpawn" "MultiplyWithRoot" null null)))

(fn `ChangeColor`
  (params (NewParam :type "Color Structure"))
  (bind _returnvalue (`PrimitiveComponent.CreateDynamicMaterialInstance` (`self.Cube`) 0 "/Game/Boss/Meshes/MI_CubeEnemy.MI_CubeEnemy" "None"))
  (`MaterialInstanceDynamic.SetVectorParameterValue` _returnvalue "Color" (`KismetMathLibrary.Conv_ColorToLinearColor` NewParam)))

(fn `UserConstructionScript`)