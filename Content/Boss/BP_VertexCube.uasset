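; Boss vertex cube that switches in and out of a protecting state by sliding its mesh along a local diagonal.
; Protect runs looping timers that push the cube outward and flash it blue for three seconds, then flags it as protecting.
; StopActions, only while protecting, resets the color, retracts the cube for a second and snaps it to origin.
; ChangeColor creates a dynamic instance of the enemy material on each call.
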(event `StopActions`
  (if (`self.Protecting`)
    (set `self.Protecting` false)
    (`self.ChangeColor` (make `Color` 0 0 0 100))
    (`KismetSystemLibrary.K2_SetTimer` null "Shrink" 0.1 true)
    (`KismetSystemLibrary.Delay` 1.0)
    (`KismetSystemLibrary.K2_PauseTimer` null "Shrink")
    (`SceneComponent.K2_SetRelativeLocation` (`self.Cube`) (0.0 0.0 0.0) false false)))

(event `Shrink`
  (bind _returnvalue_location (`KismetMathLibrary.BreakTransform` (`SceneComponent.GetRelativeTransform` (`self.Cube`))))
  (`SceneComponent.K2_SetRelativeLocation` (`self.Cube`) (+ _returnvalue_location (-9.0 -9.0 -9.0)) false false))

(event `Expand`
  (bind _returnvalue_location (`KismetMathLibrary.BreakTransform` (`SceneComponent.GetRelativeTransform` (`self.Cube`))))
  (`SceneComponent.K2_SetRelativeLocation` (`self.Cube`) (+ _returnvalue_location (3.0 3.0 3.0)) false false))

(event `ShineBlue`
  (`KismetSystemLibrary.Delay` 0.5)
  (`self.ChangeColor` (make `Color` 0 0 0 100))
  (`KismetSystemLibrary.Delay` 0.5)
  (`self.ChangeColor` (make `Color` 255 0 0 100)))

(event `Protect`
  (`KismetSystemLibrary.K2_SetTimer` null "Expand" 0.1 true)
  (`KismetSystemLibrary.K2_SetTimer` null "ShineBlue" 1.0 true false -1.0)
  (`KismetSystemLibrary.Delay` 3.0)
  (`KismetSystemLibrary.K2_PauseTimer` null "ShineBlue")
  (`KismetSystemLibrary.K2_PauseTimer` null "Expand")
  (set `self.Protecting` true))

(event `self.ReceiveBeginPlay`)

(fn `ChangeColor`
  (params (NewParam :type "Color Structure"))
  (bind _returnvalue (`PrimitiveComponent.CreateDynamicMaterialInstance` (`self.Cube`) 0 "/Game/Boss/Meshes/MI_CubeEnemy.MI_CubeEnemy" "None"))
  (`MaterialInstanceDynamic.SetVectorParameterValue` _returnvalue "Color" (`KismetMathLibrary.Conv_ColorToLinearColor` NewParam)))

(fn `UserConstructionScript`)